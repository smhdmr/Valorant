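; BP_Shutter is a shutter actor that opens and closes by scaling its Door component along Z.
; A four-value state drives Tick, which moves the scale at a rate set by MoveTime and runs only during movement.
; ToggleState starts or reverses movement, with start and stop signalled through CallMovementStarted and CallMovementStopped.
; The construction script applies the initial open or closed state, and RegisterInteractor keeps a unique list of interactors.
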(event EventTick
  (params (DeltaSeconds :type Float%20%28single-precision%29))
  (bind _door (Variables|Default|GetDoor))
  (bind _closedscale (Variables|Default|GetClosedScale))
  (bind _door_2 (Variables|Default|GetDoor))
  (bind _door_3 (Variables|Default|GetDoor))
  (bind _relativescale3d (Variables|/Script/Engine.SceneComponent|GetRelativeScale3D _door))
  (bind _relativescale3d_2 (Variables|/Script/Engine.SceneComponent|GetRelativeScale3D _door_2))
  (bind _relativescale3d_3 (Variables|/Script/Engine.SceneComponent|GetRelativeScale3D _door_3))
  (bind _returnvalue (Math|Float|NearlyEqual(Float) (.z _relativescale3d) _closedscale 1e-06))
  (switch Utilities|FlowControl|Switch|SwitchonE_ShutterState (Variables|Default|GetShutterState)
    (:NewEnumerator2
      (if (not (Math|Float|NearlyEqual(Float) (.z _relativescale3d_3) (Variables|Default|GetOpenedScale) 1e-06))
        (Transformation|SetRelativeScale3D _door_3 (Math|Vector|MakeVector (.x _relativescale3d_3) (.y _relativescale3d_3) (Math|Float|Clamp(Float) (- (.z _relativescale3d_3) (CallFunction|GetMovementAmount DeltaSeconds)) (Variables|Default|GetOpenedScale) (Variables|Default|GetClosedScale))))
        (else
          (Variables|Default|SetShutterState "NewEnumerator0")
          (Actor|Tick|SetActorTickEnabled false)
          (Default|CallMovementStopped :!label _label))))
    (:NewEnumerator3
      (if _returnvalue
        (Variables|Default|SetShutterState "NewEnumerator1")
        (Actor|Tick|SetActorTickEnabled false)
        (goto _label)
        (elif (not _returnvalue)
          (Transformation|SetRelativeScale3D _door_2 (Math|Vector|MakeVector (.x _relativescale3d_2) (.y _relativescale3d_2) (Math|Float|Clamp(Float) (+ (.z _relativescale3d_2) (CallFunction|GetMovementAmount DeltaSeconds)) (Variables|Default|GetOpenedScale) (Variables|Default|GetClosedScale)))))))))

(fn ConstructionScript
  (bind _door (Variables|Default|GetDoor))
  (bind _relativescale3d (Variables|/Script/Engine.SceneComponent|GetRelativeScale3D _door))
  (if (Variables|ShutterSettings|GetisStartingOpen)
    (Variables|Default|SetShutterState "NewEnumerator0")
    (Transformation|SetRelativeScale3D _door (Math|Vector|MakeVector (.x _relativescale3d) (.y _relativescale3d) (Variables|Default|GetOpenedScale)))
    (else
      (Variables|Default|SetShutterState "NewEnumerator1")
      (Transformation|SetRelativeScale3D _door (Math|Vector|MakeVector (.x _relativescale3d) (.y _relativescale3d) (Variables|Default|GetClosedScale)))))
  (Actor|Tick|SetActorTickEnabled false))

(fn ToggleState
  (switch Utilities|FlowControl|Switch|SwitchonE_ShutterState (Variables|Default|GetShutterState)
    (:NewEnumerator0
      (Variables|Default|SetShutterState "NewEnumerator3" :!label _label))
    (:NewEnumerator1
      (Variables|Default|SetShutterState "NewEnumerator2" :!label _label_2))
    (:NewEnumerator2
      (goto _label))
    (:NewEnumerator3
      (goto _label_2)))
  (Actor|Tick|SetActorTickEnabled true)
  (Default|CallMovementStarted))

(fn GetMovementAmount
  (params (DeltaSec :type Float%20%28single-precision%29))
  (return (/ (* DeltaSec (- (Variables|Default|GetClosedScale) (Variables|Default|GetOpenedScale))) (Variables|ShutterSettings|GetMoveTime))))

(fn RegisterInteractor
  (params (Interactor :type Interactor%20Component%20Object%20Reference))
  (Utilities|Array|AddUnique (Variables|Default|GetInteractors) Interactor))