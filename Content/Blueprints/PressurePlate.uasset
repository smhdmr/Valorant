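; Pressure plate actor that toggles a hooked shutter when a Character steps onto or off it.
; Collider begin and end overlaps swap the Top mesh between activated and deactivated materials, and both call ToggleState on HookedShutter.
; The construction script shows an unhooked material when no shutter is assigned, and overlaps then do nothing.
; Each Character overlap toggles independently, with no count of occupants.
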(event OnComponentBeginOverlap(Collider)
  (params (OverlappedComponent :type Primitive%20Component%20Object%20Reference) (OtherActor :type Actor%20Object%20Reference) (OtherComp :type Primitive%20Component%20Object%20Reference) (OtherBodyIndex :type Integer) (bFromSweep :type Boolean) (SweepResult :type Hit%20Result%20Structure%20%28by%20ref%29))
  (Utilities|IsValid (Variables|Default|GetHookedShutter)
    (:Is%20Valid
      (Utilities|Casting|CastToCharacter OtherActor)
      (Rendering|Material|SetMaterial (Variables|Default|GetTop) 0 (Variables|Materials|GetActivatedMaterial))
      (Default|ToggleState (Variables|Default|GetHookedShutter)))))

(event OnComponentEndOverlap(Collider)
  (params (OverlappedComponent :type Primitive%20Component%20Object%20Reference) (OtherActor :type Actor%20Object%20Reference) (OtherComp :type Primitive%20Component%20Object%20Reference) (OtherBodyIndex :type Integer))
  (Utilities|IsValid (Variables|Default|GetHookedShutter)
    (:Is%20Valid
      (Utilities|Casting|CastToCharacter OtherActor)
      (Rendering|Material|SetMaterial (Variables|Default|GetTop) 0 (Variables|Materials|GetDeactivatedMat))
      (Default|ToggleState (Variables|Default|GetHookedShutter)))))

(fn ConstructionScript
  (bind _top (Variables|Default|GetTop))
  (Utilities|IsValid (Variables|Default|GetHookedShutter)
    (:Is%20Valid
      (Rendering|Material|SetMaterial _top 0 (Variables|Materials|GetDeactivatedMat)))
    (:Is%20Not%20Valid
      (Rendering|Material|SetMaterial _top 0 (Variables|Materials|GetUnhookedMat)))))